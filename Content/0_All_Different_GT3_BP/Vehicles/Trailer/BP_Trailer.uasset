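; Towable trailer that hitches to a vehicle and can secure another vehicle as cargo.
; Use on the Box toggles attachment: it finds an overlapping "Hitch"-tagged component, snaps the mesh to it and constrains it to the owning BP_Master_Vehicle.
; Use on other components toggles cargo, constraining the first vehicle overlapping Cargo through a second physics constraint.
; Each state change shows a timed popup widget, replacing existing ones.
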(event `Attach`
  (for _array_element (`PrimitiveComponent.GetOverlappingComponents` (`self.Box`))
    (if (`KismetArrayLibrary.Array_Contains` (`ActorComponent.ComponentTags` _array_element) "Hitch")
      (`|ExecutionSequence`
        (:`then_0`
          (break))
        (:`then_1`
          (`SceneComponent.K2_SetWorldTransform` (`self.Mesh`) (`SceneComponent.K2_GetComponentToWorld` _array_element) false false)
          (bind _asbp_master_vehicle (cast `/Game/0_All_Different_GT3_BP/Vehicles/00_Master_Vehicle/BP_Master_Vehicle` (`ActorComponent.GetOwner` _array_element)))
          (`PhysicsConstraintComponent.SetConstrainedComponents` (`self.PhysicsConstraint`) (`self.Mesh`) "None" (`/Game/0_All_Different_GT3_BP/Vehicles/00_Master_Vehicle/BP_Master_Vehicle.Mesh` _asbp_master_vehicle) "None")
          (set `self.Is Attached` true)
          (`self.Pop-up` 3.0 "Trailer Attached!"))))))

(event `self.Use`
  (params (Component :type "ActorComponent Object Reference"))
  (if (== Component (`self.Box`))
    (if (`self.Is Attached`)
      (`self.Detach`)
      (else
        (`self.Attach`)))
    (elif (`self.Is Cargo Secured`)
      (`self.Release Cargo`)
      (else
        (`self.Secure_Cargo`)))))

(event `Detach`
  (`PhysicsConstraintComponent.BreakConstraint` (`self.PhysicsConstraint`))
  (`PrimitiveComponent.AddImpulseAtLocation` (`self.Mesh`) (0.0 0.0 0.0) (0.0 0.0 0.0) "None")
  (set `self.Is Attached` false)
  (`self.Pop-up` 3.0 "Trailer detached!"))

(event `Secure_Cargo`
  (bind _asbp_master_vehicle (cast `/Game/0_All_Different_GT3_BP/Vehicles/00_Master_Vehicle/BP_Master_Vehicle` (`|GetArrayItem` (`PrimitiveComponent.GetOverlappingActors` (`self.Cargo`) "/Game/0_All_Different_GT3_BP/Vehicles/00_Master_Vehicle/BP_Master_Vehicle.BP_Master_Vehicle_C"))))
  (`PhysicsConstraintComponent.SetConstrainedComponents` (`self.PhysicsConstraint1`) (`/Game/0_All_Different_GT3_BP/Vehicles/00_Master_Vehicle/BP_Master_Vehicle.Mesh` _asbp_master_vehicle) "None" (`self.Mesh`) "None")
  (`self.Pop-up` 3.0 "Cargo secured!")
  (set `self.Is Cargo Secured` true))

(event `Release Cargo`
  (`PhysicsConstraintComponent.BreakConstraint` (`self.PhysicsConstraint1`))
  (`self.Pop-up` 3.0 "Cargo released")
  (set `self.Is Cargo Secured` false))

(fn `Pop-up`
  (params (Duration :type "Float (double-precision)") (Text :type Text))
  (bind _foundwidgets (`WidgetBlueprintLibrary.GetAllWidgetsOfClass` "/Game/UMG/Pop-up.Pop-up_C"))
  (for _array_element _foundwidgets
    (`Widget.RemoveFromParent` _array_element))
  (bind _returnvalue (`|CreateWidget` "/Game/UMG/Pop-up.Pop-up_C" (`GameplayStatics.GetPlayerController` 0) Duration Text))
  (`UserWidget.AddToViewport` _returnvalue 0))

(fn `UserConstructionScript`)