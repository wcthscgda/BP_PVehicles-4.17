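; Racing game mode that spawns the car selected in the game instance at the player start, possesses it and runs a timed start hold.
; On BeginPlay it stores the first track spline and gathers all master vehicles, locking each with handbrake and disabled input.
; After a short delay it releases every car and shows the vehicle HUD through the player-controlled car's controller.
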(event `self.ReceiveBeginPlay`
  (bind _cars (`self.Cars`))
  (bind _asbp_game_instance (cast `/Game/BP_GameInstance` (`GameplayStatics.GetGameInstance`)))
  (bind _returnvalue (`|SpawnActorFromClass` (`/Game/BP_GameInstance.Selected Car` _asbp_game_instance) (`self.GetTransform` (`self.K2_FindPlayerStart` null)) "AdjustIfPossibleButAlwaysSpawn" "OverrideRootScale" null false true true true true true false false false false 1.0 1.5 0.0 "/Game/Vehicles/00_Master_Vehicle/Materials/M_default.M_default" "/Game/Vehicles/Camaro/Sounds/Camaro_Engine_Cue.Camaro_Engine_Cue" null))
  (`Controller.Possess` (`GameplayStatics.GetPlayerController` 0) _returnvalue)
  (bind _outactors (`GameplayStatics.GetAllActorsOfClass` "/Game/Environment/RaceTrack/BP_Track_Spline.BP_Track_Spline_C"))
  (set `self.Track` (`|GetArrayItem` _outactors))
  (bind _outactors_2 (`GameplayStatics.GetAllActorsOfClass` "/Game/Vehicles/00_Master_Vehicle/BP_Master_Vehicle.BP_Master_Vehicle_C"))
  (for _array_element _outactors_2
    (`KismetArrayLibrary.Array_Add` _cars _array_element)
    (`/Game/Vehicles/00_Master_Vehicle/BP_Master_Vehicle.Server_Handbrake` _array_element true)
    (`self.DisableInput` _array_element null))
  (`KismetSystemLibrary.Delay` 3.0)
  (for _array_element_2 _cars
    (`/Game/Vehicles/00_Master_Vehicle/BP_Master_Vehicle.Server_Handbrake` _array_element_2 false)
    (`self.EnableInput` _array_element_2 null)
    (if (`/Game/Vehicles/00_Master_Vehicle/BP_Master_Vehicle.Is Player Controlled` _array_element_2)
      (bind _asbp_controller (cast `/Game/BP_Controller` (`Pawn.GetController` _array_element_2)))
      (`/Game/BP_Controller.Show Vehicle HUD` _asbp_controller))))

(fn `UserConstructionScript`)