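; MyHUD is a vehicle HUD Blueprint meant to draw speed in km/h and current gear, with reverse in red.
; A MyGame Swap flag selects whether readings come from the owning pawn's or AiPawn's vehicle movement.
; Text scales against 1280x720, though the screen-size inputs are zero.
; DrawHUD is empty and the drawing chain is disconnected, with an unresolved pawn cast, so nothing is drawn.
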(event `self.ReceiveDrawHUD`
  (params (SizeX :type Integer) (SizeY :type Integer))
  ;[1 1 1] Calculate ratio from 720p
)

(fn `UserConstructionScript`)