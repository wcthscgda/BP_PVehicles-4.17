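; Spline-driven fence actor that builds a run of fence meshes along an editable path in its construction script.
; Each segment between adjacent spline points gets a spline mesh component, positioned by TrackStartEnd and given scaled-down roll from TrackRoll when noticeable.
; The self-resetting AdaptFenceToTerrain toggle then uses vertical line traces to move every point except the last onto hit world geometry, after the meshes are placed.
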(fn `Track Roll`
  (params (PointIndex :type Integer))
  (returns (`Start Roll` :type "Float (double-precision)") (`End Roll` :type "Float (double-precision)") (`Any Roll?` :type Boolean))
  (bind _spline (`self.Spline`))
  (bind _returnvalue (`SplineComponent.GetRollAtSplinePoint` _spline (+ PointIndex 1) "Local"))
  (bind _returnvalue_2 (`SplineComponent.GetRollAtSplinePoint` _spline PointIndex "Local"))
  (return (/ _returnvalue_2 25.0) (/ _returnvalue 25.0) (or (> (`KismetMathLibrary.Abs` _returnvalue_2) 1.0) (> (`KismetMathLibrary.Abs` _returnvalue) 1.0))))

(fn `Track Start-End`
  (params (`Lateral Offset` :type "Float (double-precision)") (PointIndex :type Integer))
  (returns (`Start Tangent` :type "Vector Structure") (`Start Location` :type "Vector Structure") (`End Tangent` :type "Vector Structure") (`End Location` :type "Vector Structure"))
  (bind _returnvalue (+ PointIndex 1))
  (bind _spline (`self.Spline`))
  (bind (_returnvalue_location _returnvalue_rotation) (`KismetMathLibrary.BreakTransform` (`SplineComponent.GetTransformAtSplinePoint` _spline PointIndex "Local" false)))
  (bind _returnvalue_2 (`KismetMathLibrary.SelectInt` _returnvalue (`KismetMathLibrary.SelectInt` 0 PointIndex) (<= _returnvalue (- (`SplineComponent.GetNumberOfSplinePoints` (`self.Spline`)) 1))))
  (bind (_returnvalue_location_2 _returnvalue_rotation_2) (`KismetMathLibrary.BreakTransform` (`SplineComponent.GetTransformAtSplinePoint` _spline _returnvalue_2 "Local" false)))
  (return (`SplineComponent.GetTangentAtSplinePoint` _spline PointIndex "Local") (+ (+ _returnvalue_location (* (`KismetMathLibrary.GetRightVector` _returnvalue_rotation) `Lateral Offset`)) (0.0 0.0 0.0)) (`SplineComponent.GetTangentAtSplinePoint` _spline _returnvalue_2 "Local") (+ (+ _returnvalue_location_2 (* (`KismetMathLibrary.GetRightVector` _returnvalue_rotation_2) `Lateral Offset`)) (0.0 0.0 0.0))))

(fn `UserConstructionScript`
  (bind _spline (`self.Spline`))
  (bind _returnvalue (- (`SplineComponent.GetNumberOfSplinePoints` (`self.Spline`)) 1))
  (bind _returnvalue_2 (- (`SplineComponent.GetNumberOfSplinePoints` _spline) 1))
  ;[1 1 1] Place Track
  (for _index (range (+ _returnvalue 1))
    (if (not (== _index _returnvalue))
      (bind _returnvalue_3 (`AddComponent|NODE_AddSplineMeshComponent-2`))
      (bind (_start_tangent _start_location _end_tangent _end_location) (`self.Track Start-End` 0.0 _index))
      (`SplineMeshComponent.SetStartAndEnd` _returnvalue_3 _start_location _start_tangent _end_location _end_tangent true)
      (bind (_start_roll _end_roll _any_roll_) (`self.Track Roll` _index))
      (if _any_roll_
        (`SplineMeshComponent.SetStartRoll` _returnvalue_3 _start_roll true)
        (`SplineMeshComponent.SetEndRoll` _returnvalue_3 _end_roll true))))
  (if (`self.Adapt Fence to Terrain`)
    (set `self.Adapt Fence to Terrain` false)
    (for _index_2 (range (+ _returnvalue_2 1))
      (if (not (== _index_2 _returnvalue_2))
        (bind _returnvalue_4 (`SplineComponent.GetLocationAtSplinePoint` _spline _index_2 "World"))
        (bind _outhit (`KismetSystemLibrary.LineTraceSingleForObjects` (+ _returnvalue_4 (0.0 0.0 50000.0)) (+ _returnvalue_4 (0.0 0.0 -50000.0)) (`|MakeArray` "ObjectTypeQuery1" "ObjectTypeQuery2" :!type "EObjectTypeQuery Enum")))
        (`SplineComponent.SetLocationAtSplinePoint` _spline _index_2 (`.Location` (`GameplayStatics.BreakHitResult` _outhit)) "World" true)))))