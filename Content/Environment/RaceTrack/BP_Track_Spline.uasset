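; Race track Blueprint that lays road spline meshes along an editable spline, optionally closed into a loop by ConnectLastToFirst.
; The construction script adds a mesh per segment, using TrackStartEnd for laterally offsettable endpoints and tangents, and TrackRoll for scaled-down banking.
; Fence rails, posts on both sides and point-index labels exist only as disconnected logic.
; BuildFences is empty, and its UpdateFences trigger is also disconnected.
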(event `Build Fences`)

(fn `Track Roll`
  (params (PointIndex :type Integer))
  (returns (`Start Roll` :type "Float (double-precision)") (`End Roll` :type "Float (double-precision)") (`Any Roll?` :type Boolean))
  (bind _spline (`self.Spline`))
  (bind _returnvalue (`SplineComponent.GetRollAtSplinePoint` _spline (+ PointIndex 1) "Local"))
  (bind _returnvalue_2 (`SplineComponent.GetRollAtSplinePoint` _spline PointIndex "Local"))
  (return (/ _returnvalue_2 25.0) (/ _returnvalue 25.0) (or (> (`KismetMathLibrary.Abs` _returnvalue_2) 1.0) (> (`KismetMathLibrary.Abs` _returnvalue) 1.0))))

(fn `Track Start-End`
  (params (`Lateral Offset` :type "Float (double-precision)") (PointIndex :type Integer))
  (returns (`Start Tangent` :type "Vector Structure") (`Start Location` :type "Vector Structure") (`End Tangent` :type "Vector Structure") (`End Location` :type "Vector Structure"))
  (bind _returnvalue (+ PointIndex 1))
  (bind _spline (`self.Spline`))
  (bind (_returnvalue_location _returnvalue_rotation) (`KismetMathLibrary.BreakTransform` (`SplineComponent.GetTransformAtSplinePoint` _spline PointIndex "Local" false)))
  (bind _returnvalue_2 (`KismetMathLibrary.SelectInt` _returnvalue (`KismetMathLibrary.SelectInt` 0 PointIndex (`self.Connect Last to First`)) (<= _returnvalue (`SplineComponent.GetNumberOfSplinePoints` (`self.Spline`)))))
  (bind (_returnvalue_location_2 _returnvalue_rotation_2) (`KismetMathLibrary.BreakTransform` (`SplineComponent.GetTransformAtSplinePoint` _spline _returnvalue_2 "Local" false)))
  (return (`SplineComponent.GetTangentAtSplinePoint` _spline PointIndex "Local") (+ _returnvalue_location (* (`KismetMathLibrary.GetRightVector` _returnvalue_rotation) `Lateral Offset`)) (`SplineComponent.GetTangentAtSplinePoint` _spline _returnvalue_2 "Local") (+ _returnvalue_location_2 (* (`KismetMathLibrary.GetRightVector` _returnvalue_rotation_2) `Lateral Offset`))))

(fn `UserConstructionScript`
  (bind _spline (`self.Spline`))
  (bind _returnvalue (- (`SplineComponent.GetNumberOfSplinePoints` _spline) 1))
  (`SplineComponent.SetClosedLoop` _spline (`self.Connect Last to First`) true)
  ;[1 1 1] Place Track
  (for _index (range (+ _returnvalue 1))
    (if (== _index _returnvalue)
      (if (`self.Connect Last to First`)
        (bind _returnvalue_2 (`AddComponent|NODE_AddSplineMeshComponent-2` :!label _label))
        (bind (_start_tangent _start_location _end_tangent _end_location) (`self.Track Start-End` 0.0 _index))
        (`SplineMeshComponent.SetStartAndEnd` _returnvalue_2 _start_location _start_tangent _end_location _end_tangent true)
        (bind (_start_roll _end_roll _any_roll_) (`self.Track Roll` _index))
        (if _any_roll_
          (`SplineMeshComponent.SetStartRoll` _returnvalue_2 _start_roll true)
          (`SplineMeshComponent.SetEndRoll` _returnvalue_2 _end_roll true)))
      (else
        (goto _label)))))