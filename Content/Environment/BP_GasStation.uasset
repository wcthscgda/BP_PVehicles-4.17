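; Gas station actor that refuels a BP_Master_Vehicle parked inside its trigger box.
; Use on the Box component stores the first overlapping vehicle and opens a Gate fed by Tick.
; While open, each tick adds fuel at a frame-rate-dependent rate and displays the percentage on a TextRender.
; Reaching full, or an end overlap matching the first overlapping vehicle, closes the gate and restores the prompt text.
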(event `self.Use`
  (params (Component :type "ActorComponent Object Reference"))
  (if (== Component (`self.Box`))
    (bind _asbp_master_vehicle (cast `/Game/Vehicles/00_Master_Vehicle/BP_Master_Vehicle` (`|GetArrayItem` (`PrimitiveComponent.GetOverlappingActors` (`self.Box1`) "/Game/Vehicles/00_Master_Vehicle/BP_Master_Vehicle.BP_Master_Vehicle_C"))))
    (`self.Open Gate`)))

(event `self.ReceiveTick`
  (params (DeltaSeconds :type "Float (single-precision)"))
  (`/Engine/EditorBlueprintResources/StandardMacros.Gate` true :!label _label
    (:`Exit`
      (bind _output_get (set `/Game/Vehicles/00_Master_Vehicle/BP_Master_Vehicle.Fuel Ammount` (+ (`/Game/Vehicles/00_Master_Vehicle/BP_Master_Vehicle.Fuel Ammount` (stale `self.Use` _asbp_master_vehicle)) 0.1) (stale `self.Use` _asbp_master_vehicle)))
      (`TextRenderComponent.K2_SetText` (`self.TextRender`) (`KismetTextLibrary.Conv_StringToText` (`KismetStringLibrary.Concat_StrStr` (`KismetStringLibrary.Conv_IntToString` (`KismetMathLibrary.Round` _output_get)) " %")))
      (if (>= _output_get 100.0)
        (`self.Close Gate`)
        (set `/Game/Vehicles/00_Master_Vehicle/BP_Master_Vehicle.Fuel Ammount` 100.0 (stale `self.Use` _asbp_master_vehicle))))))

(event `Open Gate`
  (goto _label :!via `Open`))

(event `Close Gate`
  (`TextRenderComponent.K2_SetText` (`self.TextRender`) "Press \"F\" to fuel a car.")
  (goto _label :!via `Close`))

(event `self.Box1.OnComponentEndOverlap`
  (params (OverlappedComponent :type "PrimitiveComponent Object Reference") (OtherActor :type "Actor Object Reference") (OtherComp :type "PrimitiveComponent Object Reference") (OtherBodyIndex :type Integer))
  (if (== OtherActor (`|GetArrayItem` (`PrimitiveComponent.GetOverlappingActors` (`self.Box1`) "/Game/Vehicles/00_Master_Vehicle/BP_Master_Vehicle.BP_Master_Vehicle_C")))
    (`self.Close Gate`)))

(fn `UserConstructionScript`
  (`parent.UserConstructionScript`))